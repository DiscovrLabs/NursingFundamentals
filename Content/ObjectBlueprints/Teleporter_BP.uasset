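; Teleporter actor that displays a hoverable widget and keeps itself turned toward the player's camera.
; On BeginPlay it caches the HoverableWidget from its WidgetComponent, and SetWidgetHovered forwards the hover state to that widget.
; Every Tick it rotates the whole actor with a look-at toward the camera location, giving a billboard effect.
; The teleport itself is not handled in these graphs.
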(event EventBeginPlay
  (bind _ashoverable_widget (Utilities|Casting|CastToHoverableWidget (UserInterface|GetUserWidgetObject (Variables|Default|GetWidgetComponent))))
  (Variables|Default|SetWidget _ashoverable_widget))

(event EventTick
  (params (DeltaSeconds :type Float%20%28single-precision%29))
  (Transformation|SetActorRotation (Math|Rotator|FindLookatRotation (Transformation|GetActorLocation) (Camera|GetCameraLocation (Game|GetPlayerCameraManager 0)))))

(event EventSetWidgetHovered
  (params (bHovered :type Boolean))
  (Default|SetHovered (Variables|Default|GetWidget) bHovered))

(fn ConstructionScript)